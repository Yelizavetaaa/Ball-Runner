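; BP_Crystal_01 is a crystal actor that disappears when the player pawn overlaps its sphere, apparently a pickup.
; The overlap caches several values and plays the CrystalTransform timeline, which sets location, lerps scale to zero and fades the point light before destroying the actor.
; The cached variable names do not match their values: CrystalScale holds the player's location.
; The location lerp uses zero vectors, placing the actor at world origin.
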(event OnComponentBeginOverlap(Sphere)
  (params (OverlappedComponent :type Primitive%20Component%20Object%20Reference) (OtherActor :type Actor%20Object%20Reference) (OtherComp :type Primitive%20Component%20Object%20Reference) (OtherBodyIndex :type Integer) (bFromSweep :type Boolean) (SweepResult :type Hit%20Result%20Structure%20%28by%20ref%29))
  (bind _pointlight (Variables|Default|GetPointLight))
  (if (== OtherActor (Game|Player|GetPlayerPawn 0))
    (Variables|Default|SetBallLocation (Transformation|GetActorScale3D))
    (Variables|Default|SetCrystalLight (Variables|/Script/Engine.LightComponentBase|GetIntensity (Variables|Default|GetPointLight)))
    (Variables|Default|SetCrystalScale (Transformation|GetActorLocation (Game|Player|GetPlayerPawn 0)))
    (Variables|Default|SetCrystalLocation (Transformation|GetActorLocation))
    (bind (_direction _crystallocation _crystalscale _crystallight) (Timeline|CrystalTransform Play)
      (:Update
        (Transformation|SetActorLocation (Math|Vector|Lerp(Vector) "0, 0, 0" "0, 0, 0" _crystallocation) false false)
        (Transformation|SetActorScale3D (Math|Vector|Lerp(Vector) (Variables|Default|GetCrystalScale) "0, 0, 0" _crystalscale))
        (Rendering|Components|Light|SetIntensity _pointlight (Math|Float|Lerp (Variables|/Script/Engine.LightComponentBase|GetIntensity _pointlight) 0.0 _crystallight)))
      (:Finished
        (Actor|DestroyActor)))))

(fn ConstructionScript)